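; Blueprint actor for a blue butterfly that flies along the spline of a referenced track actor.
; On BeginPlay, if flagged active, it plays a timeline scaled by a duration and begun at a start offset.
; Each update maps the timeline alpha to distance along the spline, setting world location and local-space pitch and yaw, with zero roll and a 90-degree yaw correction.
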(event Custom|movecart
  (Components|Timeline|SetPlayRate (Variables|Default|GetButterflyMover) (/ 1.0 (Variables|Default|Getduration)))
  (Components|Timeline|SetNewTime (Variables|Default|GetButterflyMover) (Variables|Default|GetButterflyStartOffset))
  (bind _alpha (Timeline|ButterflyMover Play)
    (:Update
      (Variables|Default|Setalpha _alpha)
      (Transformation|SetActorLocationAndRotation (Spline|GetLocationatDistanceAlongSpline (Variables|/Game/butterfly/BP_path.BP_path_C|Getusefulspline (Variables|Default|Gettrackreference)) (Math|Float|Lerp 0.0 (Spline|GetSplineLength (Variables|/Game/butterfly/BP_path.BP_path_C|Getusefulspline (Variables|Default|Gettrackreference))) (Variables|Default|Getalpha)) "World") (Math|Rotator|MakeRotator (- 0.0 0.0) (.Pitch (Math|Rotator|BreakRotator (Spline|GetRotationatDistanceAlongSpline (Variables|/Game/butterfly/BP_path.BP_path_C|Getusefulspline (Variables|Default|Gettrackreference)) (Math|Float|Lerp 0.0 (Spline|GetSplineLength (Variables|/Game/butterfly/BP_path.BP_path_C|Getusefulspline (Variables|Default|Gettrackreference))) (Variables|Default|Getalpha)) "Local"))) (+ (.Yaw (Math|Rotator|BreakRotator (Spline|GetRotationatDistanceAlongSpline (Variables|/Game/butterfly/BP_path.BP_path_C|Getusefulspline (Variables|Default|Gettrackreference)) (Math|Float|Lerp 0.0 (Spline|GetSplineLength (Variables|/Game/butterfly/BP_path.BP_path_C|Getusefulspline (Variables|Default|Gettrackreference))) (Variables|Default|Getalpha)) "Local"))) 9e+01))))))

(event EventBeginPlay
  (if (Variables|Default|GetActiveButterfly)
    (CallFunction|Movecart)))

(fn ConstructionScript)