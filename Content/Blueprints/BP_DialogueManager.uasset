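; Dialogue scene manager that registers with the player controller, which possesses it and uses it as the view target during conversations.
; On possession it creates the dialogue widget and dresses two talker meshes with the current characters' meshes and AnimBPs.
; Lines come from data table rows by index, driving text, speaker name, talk animation and both characters' emotions.
; A missing row triggers the controller's exit transition and removes the widget.
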(event Custom|NextDialogue
  (bind _result (Math|Integer|IncrementInt (Variables|Default|Getindex))
    (:%20%20
      (CallFunction|SetSentence _result))))

(event Custom|TransitionOutBeginPlay
  (EventDispatchers|BindEventtoDialogueAction (.PlayerController (CallFunction|GetWorldPlayerController)) (EventDispatchers|CreateEvent :!event Custom|NextDialogue))
  (UserInterface|Viewport|AddtoViewport (Variables|Default|GetDialogueUI) 0))

(event Custom|OnPosses
  (bind _playercontroller (CallFunction|GetWorldPlayerController))
  (Default|SetOutTransition _playercontroller (delegate Custom|TransitionOutBeginPlay))
  (Pawn|Possess _playercontroller self)
  ;[1 1 1] a Ranger
  (Game|Player|SetViewTargetwithBlend _playercontroller self 0.0 "VTBlend_Linear" 0.0 false)
  (Variables|Default|SetDialogue (Variables|/Game/Blueprints/BP_PC_WorldPlayerController.BP_PC_WorldPlayerController_C|GetCurrentDialogue _playercontroller))
  (bind _returnvalue (UserInterface|CreateWidget "/Game/UI/WBP_Dialogue.WBP_Dialogue_C"))
  (Variables|Default|SetDialogueUI _returnvalue)
  (bind _outrownames (DataTable|GetDataTableRowNames (Variables|Default|GetDialogue)))
  (Variables|Default|SetDialogueRowNames _outrownames)
  (CallFunction|ChangeChara (Variables|Default|GetTalker1) true (Variables|/Game/Blueprints/BP_PC_WorldPlayerController.BP_PC_WorldPlayerController_C|GetcurrentC1 _playercontroller))
  (CallFunction|ChangeChara (Variables|Default|GetTalker2) false (Variables|/Game/Blueprints/BP_PC_WorldPlayerController.BP_PC_WorldPlayerController_C|GetcurrrentC2 _playercontroller))
  (CallFunction|SetSentence (Variables|Default|Getindex)))

(event EventBeginPlay
  (Variables|/Game/Blueprints/BP_PC_WorldPlayerController.BP_PC_WorldPlayerController_C|SetDialogueManager (.PlayerController (CallFunction|GetWorldPlayerController)) self))

(event EventPossessed
  (params (NewController :type Controller%20Object%20Reference)))

(fn ConstructionScript)

(fn SetSentence
  (params (index :type Integer))
  (bind _playercontroller (CallFunction|GetWorldPlayerController))
  (bind _dialogueui (Variables|Default|GetDialogueUI))
  (bind _returnvalue (Utilities|GetDataTableRow (Variables|Default|GetDialogue) (Utilities|Array|Get(acopy) (Variables|Default|GetDialogueRowNames) index))
    (:then
      (LocalVariables|SetSentence _returnvalue)
      (LocalVariables|SetT1AnimInstance (.AsABP%20Parent%20ABP (Utilities|Casting|CastToABP_ParentABP (Components|SkeletalMesh|GetAnimInstance (Variables|Default|GetTalker1)))))
      (LocalVariables|SetT2AnimInstance (.AsABP%20Parent%20ABP (Utilities|Casting|CastToABP_ParentABP (Components|SkeletalMesh|GetAnimInstance (Variables|Default|GetTalker2)))))
      (Default|SetSentence _dialogueui (.Text (Utilities|Struct|BreakS_Dialogue (LocalVariables|GetSentence))))
      (Default|SetName _dialogueui (Utilities|Select :Index (.WhosTalking (Utilities|Struct|BreakS_Dialogue (LocalVariables|GetSentence))) :Option%200 (Variables|/Game/Blueprints/BP_DA_Character.BP_DA_Character_C|GetName (Variables|/Game/Blueprints/BP_PC_WorldPlayerController.BP_PC_WorldPlayerController_C|GetcurrentC1 _playercontroller)) :Option%201 (Variables|/Game/Blueprints/BP_DA_Character.BP_DA_Character_C|GetName (Variables|/Game/Blueprints/BP_PC_WorldPlayerController.BP_PC_WorldPlayerController_C|GetcurrrentC2 _playercontroller))))
      (Default|SetTalk (LocalVariables|GetT1AnimInstance) false)
      (Default|SetTalk (Utilities|Select :Index (.WhosTalking (Utilities|Struct|BreakS_Dialogue (LocalVariables|GetSentence))) :Option%200 (LocalVariables|GetT1AnimInstance) :Option%201 (LocalVariables|GetT2AnimInstance)) true)
      (Variables|/Game/chara_ombrette/ABP_ParentABP.ABP_ParentABP_C|SetEmotion (LocalVariables|GetT1AnimInstance) (.1StCharaEmotion (Utilities|Struct|BreakS_Dialogue (LocalVariables|GetSentence))))
      (Variables|/Game/chara_ombrette/ABP_ParentABP.ABP_ParentABP_C|SetEmotion (LocalVariables|GetT2AnimInstance) (.2CndCharaEmotion (Utilities|Struct|BreakS_Dialogue (LocalVariables|GetSentence)))))
    (:RowNotFound
      (bind _playercontroller_2 (Utilities|GetWorldPlayerCoontroller)
        (:Sucess
          (Default|TransitionfromDialogue _playercontroller_2)
          (Widget|RemovefromParent (Variables|Default|GetDialogueUI)))))))

(fn ChangeChara
  (params (talkerToChange :type Skeletal%20Mesh%20Component%20Object%20Reference%20%28by%20ref%29) (IsOne :type Boolean) (Character :type BP%20DA%20Character%20Object%20Reference))
  (Class|SkinnedMeshComponent|SetSkeletalMesh talkerToChange (Variables|/Game/Blueprints/BP_DA_Character.BP_DA_Character_C|GetSkeletal_Mesh Character) true)
  (Class|SkeletalMeshComponent|SetAnimClass talkerToChange (Variables|/Game/Blueprints/BP_DA_Character.BP_DA_Character_C|GetAnimBPClass Character))
  (Variables|/Game/chara_ombrette/ABP_ParentABP.ABP_ParentABP_C|SetIsInDialogue (.AsABP%20Parent%20ABP (Utilities|Casting|CastToABP_ParentABP (Components|SkeletalMesh|GetAnimInstance talkerToChange))) true)
  (Transformation|AddLocalRotation talkerToChange (Math|Rotator|MakeRotator 0.0 0.0 (Variables|/Game/Blueprints/BP_DA_Character.BP_DA_Character_C|GetInDialoguAngleModification Character)) false false)
  (return))