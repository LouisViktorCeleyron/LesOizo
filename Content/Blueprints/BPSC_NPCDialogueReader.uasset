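; Widget component that displays NPC dialogue in the world through a BP_W_NPCDialogue widget.
; SetSentence shows the component and passes text to the widget, EndSentence hides it, and Flip forwards to the widget.
; ResetOrientation turns it toward the player camera in pitch and yaw with zero roll.
; SetOpacity fades the widget's canvas linearly with the owner's distance from the player.
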(event Custom|SetOpacity
  (Widget|SetRenderOpacity (Variables|/Game/Blueprints/BP_W_NPCDialogue.BP_W_NPCDialogue_C|GetCanvasPanel_0 (CallFunction|GetWidget)) (- 1.0 (/ (Transformation|GetDistanceTo (Components|GetOwner) (Game|GetPlayerCharacter 0)) 2e+03))))

(fn ResetOrientation
  (bind _returnvalue (Game|GetPlayerCameraManager 0))
  (bind _self self)
  (bind _returnvalue_2 (Transformation|GetWorldLocation _self))
  (bind _returnvalue_3 (Transformation|GetActorLocation _returnvalue))
  (bind _returnvalue_4 (Math|Rotator|FindLookatRotation _returnvalue_2 _returnvalue_3))
  (bind (_roll _pitch _yaw) (Math|Rotator|BreakRotator _returnvalue_4))
  (Transformation|SetWorldRotation _self (Math|Rotator|MakeRotator 0.0 _pitch _yaw) false false))

(fn Flip
  (Default|Flip (CallFunction|GetWidget)))

(fn GetWidget
  (return (.AsBP%20W%20NPCDialogue (Utilities|Casting|CastToBP_W_NPCDialogue (UserInterface|GetUserWidgetObject)))))

(fn SetSentence
  (params (InText :type Text))
  (Rendering|SetVisibility true false)
  (Default|SetText (CallFunction|GetWidget) InText))

(fn EndSentence
  (Rendering|SetVisibility false false))