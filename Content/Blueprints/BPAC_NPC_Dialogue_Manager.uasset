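; NPC dialogue manager that plays a dialogue's sentences through an NPC reader and ends both NPC and player readers on a "STOP" ID.
; Launching stores the readers and choice widget, shows the first sentence and rebinds player controller input until the dialogue ends.
; Advancing follows only the first next-sentence ID.
; Axis input picks a choice bubble once per press, storing the answer without affecting the sentence flow.
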(fn NextSentence
  (bind _currentsentence (Variables|Default|GetCurrentSentence))
  (bind _nextsentences (Variables|/Script/oizo.Sentence|GetNextSentences _currentsentence))
  (bind _output (Utilities|Array|Get(acopy) _nextsentences))
  (if (Utilities|Enum|Equal(Enum) _output "STOP")
    (CallFunction|EndDialogue)
    (else
      (bind _returnvalue (Class|DialogueAsset|GetSentencefromID (Variables|Default|GetDialogue) _output))
      (CallFunction|SetSentence _returnvalue))))

(fn LaunchDialogue
  (params (DialogueReaderMC :type BPSC%20NPC%20Dialogue%20Reader%20Object%20Reference) (DialogueReaderNPC :type BPSC%20NPC%20Dialogue%20Reader%20Object%20Reference) (DialogueChoiceWidget :type BP%20W%20NPC%20Dialogue%20Answer%20Choice%20Object%20Reference) (Dialogue :type Dialogue%20Asset%20Object%20Reference))
  (bind _playercontroller (CallFunction|GetWorldPlayerController))
  (Variables|Default|SetDialogue Dialogue)
  (Utilities|FlowControl|Sequence
    (:then_0
      (Variables|Default|SetDialogueReaderMC DialogueReaderMC)
      (Variables|Default|SetDialogueReaderNPC DialogueReaderNPC)
      (Variables|Default|SetChoiceWidget DialogueChoiceWidget))
    (:then_1
      (CallFunction|SetSentence (Utilities|Array|Get(acopy) (Variables|/Script/oizo.DialogueAsset|GetSentencesInDialogues (Variables|Default|GetDialogue)))))
    (:then_2
      (Default|BindEventtoAction _playercontroller true (EventDispatchers|CreateEvent :!event NextSentence))
      (Default|BindMovementAxis _playercontroller (EventDispatchers|CreateEvent :!event DoNothing) (EventDispatchers|CreateEvent :!event SelectDialogueChoice)))))

(fn EndDialogue
  (bind _playercontroller (CallFunction|GetWorldPlayerController))
  (Default|EndSentence (Variables|Default|GetDialogueReaderNPC))
  (Default|EndSentence (Variables|Default|GetDialogueReaderMC))
  (EventDispatchers|UnbindEventfromActionEvent _playercontroller (EventDispatchers|CreateEvent :!event NextSentence))
  (Default|BindDefaultWorldInput _playercontroller))

(fn SelectDialogueChoice
  (params (InFloat :type Float%20%28single-precision%29))
  (if (== InFloat 0.0)
    (Variables|Default|SetIsDone false)
    (elif (not (Variables|Default|GetIsDone))
      (bind _selectedindex (Default|SelectBublle (Variables|Default|GetChoiceWidget) (Math|Float|Truncate (Math|Float|Sign(Float) InFloat))))
      (Variables|Default|SetSelectedAnswer _selectedindex)
      (Variables|Default|SetIsDone true))))

(fn DoNothing
  (params (NewParam :type Float%20%28single-precision%29)))

(fn SetSentence
  (params (Target :type Sentence%20Object%20Reference))
  (bind _output_get (Variables|Default|SetCurrentSentence Target))
  (Default|SetSentence (Variables|Default|GetDialogueReaderNPC) (Variables|/Script/oizo.Sentence|GetContent _output_get)))