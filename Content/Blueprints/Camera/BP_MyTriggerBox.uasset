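; BP_MyTriggerBox is a box trigger actor in the Camera folder that broadcasts its overlaps.
; Its Box component's begin overlap event is forwarded through the OnTriggerBoxBeginOverlap dispatcher with the full overlap data.
; The construction script sizes the Box from the BoxExtent variable.
; CopyFromTrigger makes the Box match the transform and extent of the TriggerToCopyFrom actor's collision box.
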(event OnComponentBeginOverlap(Box)
  (params (OverlappedComponent :type Primitive%20Component%20Object%20Reference) (OtherActor :type Actor%20Object%20Reference) (OtherComp :type Primitive%20Component%20Object%20Reference) (OtherBodyIndex :type Integer) (bFromSweep :type Boolean) (SweepResult :type Hit%20Result%20Structure%20%28by%20ref%29))
  (Default|CallOnTriggerBoxBeginOverlap OverlappedComponent OtherActor OtherComp OtherBodyIndex bFromSweep SweepResult))

(event EventBeginPlay)

(event Collision|EventActorBeginOverlap
  (params (OtherActor :type Actor%20Object%20Reference)))

(event EventTick
  (params (DeltaSeconds :type Float%20%28single-precision%29)))

(fn ConstructionScript
  (Components|Box|SetBoxExtent (Variables|Default|GetBox) (Variables|Shape|GetBoxExtent) false))

(fn CopyfromTrigger
  (bind _triggertocopyfrom (Variables|Default|GetTriggerToCopyFrom))
  (Transformation|SetWorldTransform (Variables|Default|GetBox) (Transformation|GetActorTransform _triggertocopyfrom) false false)
  (Components|Box|SetBoxExtent (Variables|Default|GetBox) (Variables|/Script/Engine.BoxComponent|GetBoxExtent (.AsBox%20Collision (Utilities|Casting|CastToBoxComponent (Variables|/Script/Engine.TriggerBase|GetCollisionComponent _triggertocopyfrom)))) false))