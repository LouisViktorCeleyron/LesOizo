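; BPFL_Common is a function library of shared helpers for the game.
; Getters return the world player controller, the main bird (Oiseau) character and the CastleNest game instance, cast to their project types.
; LoopedClamp wraps out-of-range integers to the opposite bound, and FaceActorToCamera turns a component toward the camera with zero roll.
; GenerateInstance creates a dynamic material on the Kiwi character's mesh, using the given zone as material index.
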(fn GetWorldPlayerController
  (bind _returnvalue (Game|GetPlayerController 0))
  (bind (_asbp_pc_world_player_controller _bsuccess) (Utilities|Casting|CastToBP_PC_WorldPlayerController _returnvalue))
  (return _asbp_pc_world_player_controller _bsuccess))

(fn GetMainOizo
  (bind _asbp_main_oiseau (Utilities|Casting|CastToBP_MainOiseau (Game|GetPlayerCharacter 0)))
  (return _asbp_main_oiseau))

(fn LoopedClamp
  (params (Value :type Integer) (Min :type Integer) (Max :type Integer))
  (return (Math|Integer|SelectInt Value (Math|Integer|SelectInt Min Max (> Value Max)) (and (>= Value Min) (<= Value Max)))))

(fn FaceActortoCamera
  (params (Target :type Scene%20Component%20Object%20Reference))
  (bind _returnvalue (Transformation|GetWorldLocation Target))
  (bind _returnvalue_2 (Game|GetPlayerCameraManager 0))
  (bind _returnvalue_3 (Transformation|GetActorLocation _returnvalue_2))
  (bind _returnvalue_4 (Math|Rotator|FindLookatRotation _returnvalue _returnvalue_3))
  (bind (_roll _pitch _yaw) (Math|Rotator|BreakRotator _returnvalue_4))
  (Transformation|SetWorldRotation Target (Math|Rotator|MakeRotator 0.0 _pitch _yaw) false false))

(fn GetCastleNestInstance
  (return (.AsCastle%20Nest%20Instance (Utilities|Casting|CastToCastleNestInstance (Game|GetGameInstance)))))

(fn GenerateInstance
  (params (KiwiCharacter :type Character%20Object%20Reference) (ZoneAInstantier :type E_KiwiShaderInstance%20Enum :default "NewEnumerator0"))
  (bind _returnvalue (Math|Conversions|ToInteger(Byte) ZoneAInstantier))
  (bind _mesh (Variables|/Script/Engine.Character|GetMesh KiwiCharacter))
  (bind _returnvalue_2 (Rendering|Material|CreateDynamicMaterialInstance _mesh _returnvalue (Rendering|Material|GetMaterial _mesh _returnvalue) "None" :!class /Script/Engine.PrimitiveComponent))
  (return _returnvalue_2))