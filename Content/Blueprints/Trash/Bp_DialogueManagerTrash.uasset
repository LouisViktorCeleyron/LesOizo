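; Dialogue manager Blueprint that plays a sequence of sentences in a widget while driving a character's facial or body emotion.
; LoadDialogue stores the dialogue, creates WBP_DialogueTrash and shows the first sentence.
; Any key press advances the index, which LoadDialogue never resets, and past the last sentence removes the widget and fires OnDialogueEnd.
; SetSentence updates the widget text and writes the first character's emotion into its ABP_ParentABP anim instance.
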(event Input|KeyboardEvents|AnyKey
  (params (Key :type Key%20Structure :default "None"))
  (:Pressed
    (Math|Integer|IncrementInt (Variables|Default|GetSentenceIndex)
      (:%20%20
        (if (>= (Variables|Default|GetSentenceIndex) (Utilities|Array|Length (Variables|/Game/Blueprints/Trash/Bp_onlydialoguetrash.Bp_onlydialoguetrash_C|GetSentences (Variables|Default|GetDialogueCurrent))))
          (Widget|RemovefromParent (Variables|Default|GetDialogueWidget))
          (Default|CallOnDialogueEnd)
          (else
            (CallFunction|SetSentence (Variables|Default|GetSentenceIndex))))))))

(fn ConstructionScript)

(fn LoadDialogue
  (params (Dialogue :type Bp%20Onlydialoguetrash%20Object%20Reference))
  (Variables|Default|SetDialogueCurrent Dialogue)
  (bind _returnvalue (UserInterface|CreateWidget "/Game/Blueprints/Trash/WBP_DialogueTrash.WBP_DialogueTrash_C"))
  (bind _output_get (Variables|Default|SetDialogueWidget _returnvalue))
  (UserInterface|Viewport|AddtoViewport _output_get 0)
  (CallFunction|SetSentence))

(fn SetSentence
  (params (SentenceIndex :type Integer))
  (bind _dialoguecurrent (Variables|Default|GetDialogueCurrent))
  (bind _sentences (Variables|/Game/Blueprints/Trash/Bp_onlydialoguetrash.Bp_onlydialoguetrash_C|GetSentences _dialoguecurrent))
  (bind _output (Utilities|Array|Get(acopy) _sentences SentenceIndex))
  (bind (_text _1stcharaemotion) (Utilities|Struct|BreakS_Dialogue _output))
  (Default|SetSentence (Variables|Default|GetDialogueWidget) _text)
  (bind _asabp_parent_abp (Utilities|Casting|CastToABP_ParentABP (Components|SkeletalMesh|GetAnimInstance (Variables|/Script/Engine.SkeletalMeshActor|GetSkeletalMeshComponent (Variables|Default|GetCharacterEmotion))))
    (:then
      (Variables|/Game/Characters/chara_Marev/ABP_ParentABP.ABP_ParentABP_C|SetEmotion _asabp_parent_abp _1stcharaemotion))
    (:CastFailed
      (Development|PrintString "Hello"))))