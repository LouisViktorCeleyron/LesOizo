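; BP_DialogueManager is a possessable dialogue stage that shows two-character conversations and registers itself with the player controller.
; On possession setup, it becomes the view target, loads the current dialogue table's row names, creates WBP_Dialogue and dresses both talkers with mirrored facing.
; NextDialogue advances the index into SetSentence, whose entry is unwired, leaving its text, talk and emotion updates and EndDialogue call unreachable.
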(event Custom|NextDialogue
  (bind _result (Math|Integer|IncrementInt (Variables|Default|Getindex))
    (:%20%20
      (CallFunction|SetSentence _result))))

(event Custom|TransitionOutBeginPlay
  (EventDispatchers|BindEventtoDialogueAction (.PlayerController (CallFunction|GetWorldPlayerController)) (EventDispatchers|CreateEvent :!event Custom|NextDialogue))
  (UserInterface|Viewport|AddtoViewport (Variables|Default|GetDialogueUI) 0))

(event Custom|OnPosses
  (bind _playercontroller (CallFunction|GetWorldPlayerController))
  (Default|SetOutTransition _playercontroller (delegate Custom|TransitionOutBeginPlay))
  (Pawn|Possess _playercontroller self)
  ;[1 1 1] a Ranger
  (Game|Player|SetViewTargetwithBlend _playercontroller self 0.0 "VTBlend_Linear" 0.0 false)
  (Variables|Default|SetDialogue (Variables|/Game/Blueprints/General/BP_PC_WorldPlayerController.BP_PC_WorldPlayerController_C|GetCurrentDialogue _playercontroller))
  (bind _returnvalue (UserInterface|CreateWidget "/Game/UI/WBP_Dialogue.WBP_Dialogue_C"))
  (Variables|Default|SetDialogueUI _returnvalue)
  (bind _outrownames (DataTable|GetDataTableRowNames (Variables|Default|GetDialogue)))
  (Variables|Default|SetDialogueRowNames _outrownames)
  (CallFunction|ChangeChara (Variables|Default|GetTalker1) true (Variables|/Game/Blueprints/General/BP_PC_WorldPlayerController.BP_PC_WorldPlayerController_C|GetcurrentC1 _playercontroller))
  (CallFunction|ChangeChara (Variables|Default|GetTalker2) false (Variables|/Game/Blueprints/General/BP_PC_WorldPlayerController.BP_PC_WorldPlayerController_C|GetcurrrentC2 _playercontroller))
  (CallFunction|SetSentence (Variables|Default|Getindex)))

(event EventBeginPlay
  (Variables|/Game/Blueprints/General/BP_PC_WorldPlayerController.BP_PC_WorldPlayerController_C|SetDialogueManager (.PlayerController (CallFunction|GetWorldPlayerController)) self))

(event EventPossessed
  (params (NewController :type Controller%20Object%20Reference)))

(fn ConstructionScript
  (Variables|Default|SetOriginalRotator (Variables|/Script/Engine.SceneComponent|GetRelativeRotation (Variables|Default|GetTalker1))))

(fn SetSentence
  (params (index :type Integer)))

(fn ChangeChara
  (params (talkerToChange :type Skeletal%20Mesh%20Component%20Object%20Reference%20%28by%20ref%29) (IsOne :type Boolean) (Character :type BP%20DA%20Character%20Object%20Reference))
  (bind _originalrotator (Variables|Default|GetOriginalRotator))
  (bind _returnvalue (Components|SkeletalMesh|GetAnimInstance talkerToChange))
  (bind (_roll _pitch _yaw) (Math|Rotator|BreakRotator _originalrotator))
  (bind _returnvalue_2 (select IsOne 1.0 -1.0))
  (bind (_asabp_parent_abp _bsuccess) (Utilities|Casting|CastToABP_ParentABP _returnvalue))
  (Class|SkinnedMeshComponent|SetSkeletalMesh talkerToChange (Variables|/Game/Blueprints/DataAssets/BP_DA_Character.BP_DA_Character_C|GetSkeletal_Mesh Character) true)
  (Class|SkeletalMeshComponent|SetAnimClass talkerToChange (Variables|/Game/Blueprints/DataAssets/BP_DA_Character.BP_DA_Character_C|GetAnimBPClass Character))
  (Variables|/Game/Characters/chara_Marev/ABP_ParentABP.ABP_ParentABP_C|SetIsInDialogue _asabp_parent_abp _bsuccess)
  (Transformation|SetRelativeRotation talkerToChange (Math|Rotator|MakeRotator _roll _pitch (* (+ _yaw (Variables|/Game/Blueprints/DataAssets/BP_DA_Character.BP_DA_Character_C|GetInDialoguAngleModification Character) (* (/ (+ _returnvalue_2 -1.0) -2.0) 1.8e+02)) _returnvalue_2)) false false)
  (return))

(fn EndDialogue
  (bind _playercontroller (Utilities|GetWorldPlayerCoontroller)
    (:Sucess
      (Default|TransitionfromDialogue _playercontroller)
      (Widget|RemovefromParent (Variables|Default|GetDialogueUI))
      (Variables|Default|Setindex 0))))