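; Actor component that runs NPC dialogues, stepping through a Dialogue's sentences and ending when no next one exists.
; Each sentence fires its action and displays on either the main character's or the NPC's reader.
; Choice sentences fill a three-answer widget, where debounced axis input picks the branch by setting the next-sentence index.
; Launching rebinds player controller input for dialogue, and ending restores default world input.
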(fn NextSentence
  (ChoiceStuff|DisableChoiceParameter)
  (bind _returnvalue (Class|DialogueAsset|GetNextSentencefrom (Variables|Default|GetDialogue) (Variables|Default|GetCurrentSentence))
    (:SentenceFound
      (CallFunction|SetSentence _returnvalue))
    (:SentenceNull
      (CallFunction|EndDialogue))))

(fn LaunchDialogue
  (params (DialogueReaderMC :type BPSC%20NPC%20Dialogue%20Reader%20Object%20Reference) (DialogueReaderNPC :type BPSC%20NPC%20Dialogue%20Reader%20Object%20Reference) (DialogueChoiceWidget :type BP%20W%20NPC%20Dialogue%20Answer%20Choice%20Object%20Reference) (DialogueLauncherForReset :type BP%20BC%20I%20Launch%20Dialogue%20Object%20Reference) (Dialogue :type Dialogue%20Asset%20Object%20Reference))
  (bind _playercontroller (CallFunction|GetWorldPlayerController))
  (Variables|Default|SetDialogue Dialogue)
  (Variables|Default|SetDialogueLauncher DialogueLauncherForReset)
  (Utilities|FlowControl|Sequence
    (:then_0
      (Variables|Default|SetDialogueReaderMC DialogueReaderMC)
      (Variables|Default|SetDialogueReaderNPC DialogueReaderNPC)
      (Variables|Default|SetChoiceWidget DialogueChoiceWidget))
    (:then_1
      (CallFunction|SetSentence (Utilities|Array|Get(acopy) (Variables|/Script/oizo.DialogueAsset|GetSentencesInDialogues (Variables|Default|GetDialogue)))))
    (:then_2
      (Default|BindEventtoAction _playercontroller true (EventDispatchers|CreateEvent :!event NextSentence))
      (Default|BindMovementAxis _playercontroller (EventDispatchers|CreateEvent :!event DoNothing) (EventDispatchers|CreateEvent :!event SelectDialogueChoice)))))

(fn EndDialogue
  (bind _playercontroller (CallFunction|GetWorldPlayerController))
  (Default|EndSentence (Variables|Default|GetDialogueReaderNPC))
  (Default|EndSentence (Variables|Default|GetDialogueReaderMC))
  (Default|BindDefaultWorldInput _playercontroller)
  (Default|BindEventtoAction _playercontroller true (EventDispatchers|CreateEvent (Variables|Default|GetDialogueLauncher) :!event LaunchAction)))

(fn SelectDialogueChoice
  (params (InFloat :type Float%20%28single-precision%29))
  (if (== InFloat 0.0)
    (Variables|Default|SetIsDone false)
    (elif (not (Variables|Default|GetIsDone))
      (bind _selectedindex (Default|SelectBublle (Variables|Default|GetChoiceWidget) (Math|Float|Truncate (Math|Float|Sign(Float) InFloat))))
      (bind _aschoice_sentence (Utilities|Casting|CastToChoiceSentence (Variables|Default|GetCurrentSentence)))
      (Variables|/Script/oizo.ChoiceSentence|SetNextSentencesIndex _aschoice_sentence _selectedindex)
      (Variables|Default|SetIsDone true))))

(fn DoNothing
  (params (NewParam :type Float%20%28single-precision%29)))

(fn SetSentence
  (params (Target :type Sentence%20Object%20Reference))
  (bind _output_get (Variables|Default|SetCurrentSentence Target))
  (LocalVariables|SetContent (Variables|/Script/oizo.Sentence|GetContent _output_get))
  (Class|Sentence|ActionCalledwithSentence _output_get (.PlayerController (CallFunction|GetWorldPlayerController)))
  (Utilities|FlowControl|Sequence
    (:then_0
      (Default|EndSentence (Variables|Default|GetDialogueReaderNPC))
      (Default|EndSentence (Variables|Default|GetDialogueReaderMC)))
    (:then_1
      (LocalVariables|SetCurrentReader (select (Variables|/Script/oizo.Sentence|GetIsMainCharacter (Variables|Default|GetCurrentSentence)) (Variables|Default|GetDialogueReaderMC) (Variables|Default|GetDialogueReaderNPC))))
    (:then_2
      (Default|SetSentence (LocalVariables|GetCurrentReader) (LocalVariables|GetContent)))))

(fn EnableChoiceParameter
  (bind _choicewidget (Variables|Default|GetChoiceWidget))
  (Widget|SetVisibility _choicewidget "Visible")
  (Default|SelectBublle _choicewidget)
  (for _index (range 0 2)
    (bind _aschoice_sentence (Utilities|Casting|CastToChoiceSentence (Variables|Default|GetCurrentSentence)))
    (bind _returnvalue (Class|ChoiceSentence|GetAnswerNextSentenceDuoatIndex _aschoice_sentence _index))
    (Default|SetText (Variables|Default|GetChoiceWidget) (.AnswerContent (Utilities|Struct|BreakAnswerNextSentenceDuo _returnvalue)) _index)))

(fn DisableChoiceParameter
  (bind _choicewidget (Variables|Default|GetChoiceWidget))
  (if (Utilities|Enum|Equal(Enum) (Widget|GetVisibility _choicewidget) "Visible")
    (Widget|SetVisibility _choicewidget "Hidden")))