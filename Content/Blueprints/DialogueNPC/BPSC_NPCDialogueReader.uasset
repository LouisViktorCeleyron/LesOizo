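; BPSC_NPCDialogueReader is a widget component that displays an NPC's dialogue sentences through its BP_W_NPCDialogue widget.
; It starts hidden, shows itself when SetSentence passes in text, and hides again on EndSentence.
; SetOpacity fades the widget's canvas linearly with the owner's distance from the player character, and Flip forwards to the widget.
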(event Custom|SetOpacity
  (Widget|SetRenderOpacity (Variables|/Game/Blueprints/BP_W_NPCDialogue.BP_W_NPCDialogue_C|GetCanvasPanel_0 (CallFunction|GetWidget)) (- 1.0 (/ (Transformation|GetDistanceTo (Components|GetOwner) (Game|GetPlayerCharacter 0)) 2e+03))))

(event EventBeginPlay
  (Rendering|SetVisibility false true))

(fn Flip
  (Default|Flip (CallFunction|GetWidget)))

(fn GetWidget
  (return (.AsBP%20W%20NPCDialogue (Utilities|Casting|CastToBP_W_NPCDialogue (UserInterface|GetUserWidgetObject)))))

(fn SetSentence
  (params (InText :type Text))
  (Rendering|SetVisibility true true)
  (Default|SetText (CallFunction|GetWidget) InText))

(fn EndSentence
  (Rendering|SetVisibility false true))