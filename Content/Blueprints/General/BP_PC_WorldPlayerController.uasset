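; World player controller that routes Enhanced Input and switches between exploration and dialogue.
; Movement and interact inputs fire rebindable dispatchers, with interact going to a separate dialogue action and movement suppressed during dialogue.
; BeginPlay loads the dialogue level as a distant level instance and creates the transition widget.
; Dialogue transitions play that widget with bound callbacks, storing the BP_MainOiseau pawn for later repossession with a camera blend.
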(event Custom|StopMoving
  (params (CanMove? :type Boolean))
  (if CanMove?
    _))

(event Input|EnhancedActionEvents|EnhancedInputActionInterract
  (params (ActionValue :type Boolean) (ElapsedSeconds :type Float%20%28double-precision%29) (TriggeredSeconds :type Float%20%28double-precision%29) (InputAction :type Input%20Action%20Object%20Reference :default "/Game/Blueprints/Input/Interract.Interract"))
  (if (Variables|Default|GetIsDialogue)
    (Default|CallDialogueAction)
    (else
      (Default|CallActionEvent))))

(event EventBeginPlay
  (|CallParentFunction)
  (Utilities|FlowControl|Sequence
    (:then_0
      (CallFunction|LoadDialogueLevel)
      (bind _returnvalue (UserInterface|CreateWidget "/Game/UI/WBP_Transition.WBP_Transition_C"))
      (Variables|Default|SetTransition _returnvalue)
      (Variables|Default|SetbShowMouseCursor true)
      (Class|CastlenestPlayerController|AddInventorytoViewPort))
    (:then_1
      (Binder|BindEventtoLoadChoice))
    (:then_2
      (Input|AddMappingContext (PlayerController|LocalPlayerSubsystems|GetEnhancedInputLocalPlayerSubsystem self) "/Game/Blueprints/Input/NewInputMappingContext.NewInputMappingContext" 0 "(bIgnoreAllPressedKeysUntilRelease=True,bForceImmediately=False,bNotifyUserSettings=False)"))))

(event Input|KeyboardEvents|P
  (params (Key :type Key%20Structure :default "None")))

(event Input|EnhancedActionEvents|EnhancedInputActionMovement
  (params (ActionValue :type Vector%202D%20Structure) (ElapsedSeconds :type Float%20%28double-precision%29) (TriggeredSeconds :type Float%20%28double-precision%29) (InputAction :type Input%20Action%20Object%20Reference :default "/Game/Blueprints/Input/Movement.Movement"))
  (bind (_x _y) (Math|Vector2D|BreakVector2D ActionValue))
  (bind _isdialogue (Variables|Default|GetIsDialogue))
  (bind _canmove (Variables|Default|GetCanMove))
  (bind _returnvalue (not _isdialogue))
  (bind _returnvalue_2 (and _returnvalue _canmove))
  (Utilities|FlowControl|Sequence
    (:then_0
      (if _returnvalue_2
        (Default|CallAxisMoveRight _x)))
    (:then_1
      (if _returnvalue_2
        (Default|CallAxisMoveForward _y)))))

(fn ConstructionScript)

(fn TransitiontoDialogue
  (params (CurrentDialogue :type Data%20Table%20Object%20Reference) (currentC1 :type BP%20DA%20Character%20Object%20Reference) (currrentC2 :type BP%20DA%20Character%20Object%20Reference))
  (bind _transition (Variables|Default|GetTransition))
  (Utilities|FlowControl|Sequence
    (:then_0
      (Variables|Default|SetIsDialogue true)
      (Variables|Default|SetCurrentDialogue CurrentDialogue)
      (Variables|Default|SetLastPawnControlled (.AsBP%20Main%20Oiseau (Utilities|Casting|CastToBP_MainOiseau (Game|Player|GetPlayerPawn 0)))))
    (:then_1
      (UserInterface|Viewport|AddtoViewport (Variables|Default|GetTransition) 0)
      (EventDispatchers|BindEventtoIn _transition (EventDispatchers|CreateEvent (Variables|Default|GetDialogueManager) :!event OnPosses))
      (Default|Playin _transition))
    (:then_2
      (Variables|Default|SetcurrentC1 currentC1)
      (Variables|Default|SetcurrrentC2 currrentC2))))

(fn SetOutTransition
  (params (Event :type Delegate%20%28by%20ref%29))
  (EventDispatchers|BindEventtoOut (Variables|Default|GetTransition) Event))

(fn TransitionfromDialogue
  (Utilities|FlowControl|Sequence
    (:then_0
      (Variables|Default|SetIsDialogue false)
      (EventDispatchers|BindEventtoIn (Variables|Default|GetTransition) (EventDispatchers|CreateEvent :!event PossesWorldPlayer)))
    (:then_1
      (UserInterface|Viewport|AddtoViewport (Variables|Default|GetTransition) 0)
      (Default|Playin (Variables|Default|GetTransition)))))

(fn LoadDialogueLevel
  (Class|LevelStreamingDynamic|LoadLevelInstancebySoftObjectPtr "/Game/maps/Dialogue.Dialogue" "10000.000000,10000.000000,10000.000000" "0, 0, 0" "" 0 false))

(fn PossesWorldPlayer
  (Pawn|Possess (Variables|Default|GetLastPawnControlled))
  (Game|Player|SetViewTargetwithBlend (Variables|/Game/Blueprints/General/BP_MainOiseau.BP_MainOiseau_C|GetCurrentCamera (Variables|Default|GetLastPawnControlled)) 1.0 "VTBlend_Linear" 0.0 false))

(fn BindEventtoAction
  (params (Reset? :type Boolean) (Event :type Delegate%20%28by%20ref%29))
  (if Reset?
    (EventDispatchers|UnbindallEventsfromActionEvent))
  (EventDispatchers|BindEventtoActionEvent Event))

(fn BindMovementAxis
  (params (MoveForward :type Delegate%20%28by%20ref%29) (MoveRight :type Delegate%20%28by%20ref%29))
  (EventDispatchers|UnbindallEventsfromAxisMoveRight)
  (EventDispatchers|UnbindallEventsfromAxisMoveForward)
  (EventDispatchers|BindEventtoAxisMoveForward MoveForward)
  (EventDispatchers|BindEventtoAxisMoveRight MoveRight))

(fn BindDefaultWorldInput
  (Binder|BindMovementAxis (EventDispatchers|CreateEvent (.AsBP%20Main%20Oiseau (Utilities|Casting|CastToBP_MainOiseau (Game|Player|GetPlayerPawn 0))) :!event MoveForward) (EventDispatchers|CreateEvent (.AsBP%20Main%20Oiseau (Utilities|Casting|CastToBP_MainOiseau (Game|Player|GetPlayerPawn 0))) :!event MoveRight)))

(fn BindEventtoLoadChoice
  (Development|PrintString "Hello")
  (bind _asbp_main_oiseau (Utilities|GetMainOizo)
    (:then
      (EventDispatchers|BindEventtoCalltoCreateDialogueChoice (EventDispatchers|CreateEvent (Variables|/Game/Blueprints/General/BP_MainOiseau.BP_MainOiseau_C|GetBPAC_NPC_Dialogue_Manager _asbp_main_oiseau) :!event EnableChoiceParameter)))))

(fn GetPlayerControllerasMainOizo
  (bind _returnvalue (Game|GetPlayerCharacter 0))
  (bind (_asbp_main_oiseau _bsuccess) (Utilities|Casting|CastToBP_MainOiseau _returnvalue))
  (return _asbp_main_oiseau _bsuccess))