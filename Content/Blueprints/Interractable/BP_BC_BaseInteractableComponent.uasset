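; Base interactable component that lets the BP_MainOiseau player trigger an action while overlapping an interactable.
; Overlap start and end events cast the other actor to the bird, store it as PlayerCharacter, then bind or unbind an event on the world player controller's action.
; LaunchAction passes the stored character to Action, an empty function that serves as the hook for child-specific behavior.
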(event EventBeginPlay)

(event EventTick
  (params (DeltaSeconds :type Float%20%28single-precision%29)))

(event EventOnStartInteractiveOverlapped
  (params (overlappedComp :type Primitive%20Component%20Object%20Reference) (other :type Actor%20Object%20Reference) (otherComp :type Primitive%20Component%20Object%20Reference) (otherBodyIndex :type Integer) (bFromSweep :type Boolean) (sweepResult :type Hit%20Result%20Structure%20%28by%20ref%29))
  (bind (_playercontroller _bsuccess) (CallFunction|GetWorldPlayerController))
  (bind _asbp_main_oiseau (Utilities|Casting|CastToBP_MainOiseau other))
  (Variables|Default|SetPlayerCharacter _asbp_main_oiseau)
  (if _bsuccess
    (Default|BindEventtoAction _playercontroller true (EventDispatchers|CreateEvent :!event LaunchAction))))

(event EventOnEndInteractiveOverlapped
  (params (overlappedComponent :type Primitive%20Component%20Object%20Reference) (otherActor :type Actor%20Object%20Reference) (otherComp :type Primitive%20Component%20Object%20Reference) (otherBodyIndex :type Integer))
  (bind (_playercontroller _bsuccess) (CallFunction|GetWorldPlayerController))
  (bind _asbp_main_oiseau (Utilities|Casting|CastToBP_MainOiseau otherActor))
  (Variables|Default|SetPlayerCharacter _asbp_main_oiseau)
  (if _bsuccess
    (EventDispatchers|UnbindEventfromActionEvent _playercontroller (EventDispatchers|CreateEvent :!event LaunchAction))))

(fn LaunchAction
  (CallFunction|Action (Variables|Default|GetPlayerCharacter)))

(fn Action
  (params (MainOizo :type BP%20Main%20Oiseau%20Object%20Reference)))