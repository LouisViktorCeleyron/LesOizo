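; Interaction component for NPC characters that starts a dialogue between the player character (MainOizo) and its owning NPC.
; On BeginPlay it caches its owner as the NPC to talk with.
; Its Action event calls the player's dialogue manager with both dialogue readers, the player's answer-choice widget and itself as launcher for reset.
; The dialogue to play comes from GetDialogueToLaunch, which returns the DialogueToLaunch variable.
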(event EventBeginPlay
  (|CallParentFunction)
  (bind _asbp_npc_character (Utilities|Casting|CastToBP_NPC_Character (Components|GetOwner)))
  (Variables|Default|SetNPCToTalkWith _asbp_npc_character))

(event EventTick
  (params (DeltaSeconds :type Float%20%28single-precision%29))
  (|CallParentFunction DeltaSeconds) ; This node is disabled and will not be called.\nDrag off pins to build functionality.
)

(event EventAction
  (params (MainOizo :type BP%20Main%20Oiseau%20Object%20Reference))
  (Default|LaunchDialogue (Variables|/Game/Blueprints/General/BP_MainOiseau.BP_MainOiseau_C|GetBPAC_NPC_Dialogue_Manager MainOizo) (Variables|/Game/Blueprints/General/BP_MainOiseau.BP_MainOiseau_C|GetBPSC_NPCDialogueReader MainOizo) (Variables|/Game/Blueprints/BP_NPC_Character.BP_NPC_Character_C|GetBPSC_NPCDialogueReader1 (Variables|Default|GetNPCToTalkWith)) (.AsBP%20W%20NPC%20Dialogue%20Answer%20Choice (Utilities|Casting|CastToBP_W_NPC_DialogueAnswerChoice (UserInterface|GetUserWidgetObject (Variables|/Game/Blueprints/General/BP_MainOiseau.BP_MainOiseau_C|GetBPSC_NPC_DialogueChoice MainOizo)))) self (CallFunction|GetDialoguetoLaunch)))

(fn GetDialoguetoLaunch
  (return (Variables|Default|GetDialogueToLaunch)))