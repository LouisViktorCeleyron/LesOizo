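; Interactable Blueprint that chooses which dialogue to launch based on game switch states.
; GetDialogueToLaunch loops over a map of switches, reading each current value from the CastleNest instance.
; It returns the dialogue of the first switch matching its expected boolean, or the default dialogue when none match.
; The event graph holds only disabled BeginPlay and Tick stubs.
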(event EventBeginPlay
  (|CallParentFunction) ; This node is disabled and will not be called.\nDrag off pins to build functionality.
)

(event EventTick
  (params (DeltaSeconds :type Float%20%28single-precision%29))
  (|CallParentFunction DeltaSeconds) ; This node is disabled and will not be called.\nDrag off pins to build functionality.
)

(fn GetDialoguetoLaunch
  (Utilities|FlowControl|Sequence
    (:then_0
      (bind _keys (Utilities|Map|Keys (Variables|Default|GetDialoguesToLaunchWithSwithches)))
      (for _array_element _keys
        (bind _returnvalue (Class|CastleNestInstance|GetSwitchValue (CallFunction|GetCastleNestInstance) _array_element))
        (if (and (.ReturnValue (Utilities|Map|Find (Variables|Default|GetDialoguesToLaunchWithSwithches) _array_element)) (Math|Boolean|Equal(Boolean) _returnvalue (Utilities|Struct|BreakSwitch (.SwitchValueExpected (Utilities|Struct|BreakF_SwitchDialogueAssociation (.Value (Utilities|Map|Find (Variables|Default|GetDialoguesToLaunchWithSwithches) _array_element)))))))
          (return (.Dialogue (Utilities|Struct|BreakF_SwitchDialogueAssociation (.Value (Utilities|Map|Find (Variables|Default|GetDialoguesToLaunchWithSwithches) _array_element))))))))
    (:then_1
      (return (Variables|Default|GetDefaultDialogueToLaunch)))))